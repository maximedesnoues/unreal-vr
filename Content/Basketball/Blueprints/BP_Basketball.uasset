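; BP_Basketball is a grabbable, throwable basketball actor driven by motion controllers.
; A GrabComponent toggles the IsHeld flag on grab and drop.
; On drop, if the Sphere simulates physics, it takes the controller's linear velocity, scaled by a throw multiplier and clamped to a maximum speed.
; Angular velocity is likewise scaled and clamped to give spin, applied only when the linear velocity read succeeds.
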(event OnGrabbed(GrabComponent)
  (Variables|Default|SetisHeld true))

(event OnDropped(GrabComponent)
  (bind _grabcomponent (Variables|Default|GetGrabComponent))
  (bind _motioncontrollerref (Variables|/Game/XRFramework/Blueprints/BP_GrabComponent.BP_GrabComponent_C|GetMotionControllerRef _grabcomponent))
  (bind (_outlinearvelocity _returnvalue) (Class|MotionControllerComponent|GetLinearVelocity _motioncontrollerref))
  (bind (_outangularvelocity _returnvalue_2) (Class|MotionControllerComponent|GetAngularVelocity _motioncontrollerref))
  (bind (_roll _pitch _yaw) (Math|Rotator|BreakRotator _outangularvelocity))
  (Variables|Default|SetisHeld false)
  (Utilities|IsValid (Variables|/Game/XRFramework/Blueprints/BP_GrabComponent.BP_GrabComponent_C|GetMotionControllerRef (Variables|Default|GetGrabComponent))
    (:Is%20Valid
      (if (Physics|IsSimulatingPhysics (Variables|Default|GetSphere) "None")
        (if _returnvalue
          (Physics|SetPhysicsLinearVelocity (Variables|Default|GetSphere) (Math|Vector|ClampVectorSize (* _outlinearvelocity (Variables|Default|GetthrowMultiplier)) 0.0 (Variables|Default|GetmaxThrowSpeed)) false "None")
          (if _returnvalue_2
            (Class|PrimitiveComponent|SetPhysicsAngularVelocityinDegrees (Variables|Default|GetSphere) (Math|Vector|ClampVectorSize (* (Math|Vector|MakeVector _roll _pitch _yaw) (Variables|Default|GetangularMultiplier)) 0.0 (Variables|Default|GetmaxAngularSpeed)) false "None")))))))

(event EventBeginPlay)

(event Collision|EventActorBeginOverlap
  (params (OtherActor :type Actor%20Object%20Reference)))

(event EventTick
  (params (DeltaSeconds :type Float%20%28single-precision%29)))

(fn ConstructionScript)
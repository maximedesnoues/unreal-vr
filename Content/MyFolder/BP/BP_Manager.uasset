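; BP_Manager is a scoring manager that tracks which of three zones the XR pawn last entered and awards points accordingly.
; Overlap events on three zone components check for BP_XRPawn and set the CurrentZone enum.
; FPoints switches on that zone, adds a larger amount for higher-numbered zones to CurrentPoint, and prints the running total.
; Nothing in this Blueprint calls FPoints.
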(event OnComponentBeginOverlap(Zone1)
  (params (OverlappedComponent :type Primitive%20Component%20Object%20Reference) (OtherActor :type Actor%20Object%20Reference) (OtherComp :type Primitive%20Component%20Object%20Reference) (OtherBodyIndex :type Integer) (bFromSweep :type Boolean) (SweepResult :type Hit%20Result%20Structure%20%28by%20ref%29))
  (Utilities|Casting|CastToBP_XRPawn OtherActor)
  (Variables|Default|SetcurrentZone "NewEnumerator0"))

(event OnComponentBeginOverlap(Zone2)
  (params (OverlappedComponent :type Primitive%20Component%20Object%20Reference) (OtherActor :type Actor%20Object%20Reference) (OtherComp :type Primitive%20Component%20Object%20Reference) (OtherBodyIndex :type Integer) (bFromSweep :type Boolean) (SweepResult :type Hit%20Result%20Structure%20%28by%20ref%29))
  (Utilities|Casting|CastToBP_XRPawn OtherActor)
  (Variables|Default|SetcurrentZone "NewEnumerator1"))

(event OnComponentBeginOverlap(Zone3)
  (params (OverlappedComponent :type Primitive%20Component%20Object%20Reference) (OtherActor :type Actor%20Object%20Reference) (OtherComp :type Primitive%20Component%20Object%20Reference) (OtherBodyIndex :type Integer) (bFromSweep :type Boolean) (SweepResult :type Hit%20Result%20Structure%20%28by%20ref%29))
  (Utilities|Casting|CastToBP_XRPawn OtherActor)
  (Variables|Default|SetcurrentZone "NewEnumerator2"))

(fn ConstructionScript)

(fn FPoints
  (switch Utilities|FlowControl|Switch|SwitchonE_Zone (Variables|Default|GetcurrentZone)
    (:NewEnumerator0
      ;[0.15 0.15 0.15 0.5] Zone 1
      (bind _output_get (Variables|Default|SetcurrentPoint (+ (Variables|Default|GetcurrentPoint) 1)))
      (Development|PrintString (Utilities|String|ToString(Integer) _output_get)))
    (:NewEnumerator1
      ;[0.15 0.15 0.15 0.5] Zone 2
      (bind _output_get_2 (Variables|Default|SetcurrentPoint (+ (Variables|Default|GetcurrentPoint) 2)))
      (Development|PrintString (Utilities|String|ToString(Integer) _output_get_2)))
    (:NewEnumerator2
      ;[0.15 0.15 0.15 0.5] Zone 3
      (bind _output_get_3 (Variables|Default|SetcurrentPoint (+ (Variables|Default|GetcurrentPoint) 3)))
      (Development|PrintString (Utilities|String|ToString(Integer) _output_get_3)))))